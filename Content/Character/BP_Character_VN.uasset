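; BP_Character_VN is a character Blueprint providing basic player look, movement, crouch and jump controls.
; Input axes drive controller yaw and pitch, plus movement along the actor's forward and right vectors, scaled by MoveSpeed and frame delta time.
; Crouch is held, gated by CanCrouch, and Jump calls the built-in function.
; Disconnected nodes for an upward impulse and for spawning an inventory and attached gun never run.
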(event `self.ReceiveBeginPlay`
  ;[1 1 1] Event BeginPlay
)

(event `InputAxis|Turn`
  (params (AxisValue :type "Float (single-precision)"))
  ;[1 1 1] Events Turn
  (`self.AddControllerYawInput` AxisValue))

(event `InputAxis|TurnY`
  (params (AxisValue :type "Float (single-precision)"))
  ;[1 1 1] Events Turn
  (`self.AddControllerPitchInput` AxisValue))

(event `InputAction|Crouch`
  (params (Key :type "Key Structure"))
  ;[1 1 1] Events crouch_jump
  (:`Pressed`
    (if (`self.CanCrouch`)
      (`self.Crouch`)))
  (:`Released`
    (`self.UnCrouch`)))

(event `InputAction|Jump`
  (params (Key :type "Key Structure"))
  ;[1 1 1] Events crouch_jump
  (:`Pressed`
    (`self.Jump`)))

(event `InputAxis|MoveRight`
  (params (AxisValue :type "Float (single-precision)"))
  ;[1 1 1] Moving
  (`self.AddMovementInput` (* (`self.GetActorRightVector`) (* (`GameplayStatics.GetWorldDeltaSeconds`) (`self.MoveSpeed`))) AxisValue))

(event `InputAxis|MoveForward`
  (params (AxisValue :type "Float (single-precision)"))
  ;[1 1 1] Moving
  (`self.AddMovementInput` (* (`self.GetActorForwardVector`) (* (`GameplayStatics.GetWorldDeltaSeconds`) (`self.MoveSpeed`))) AxisValue))

(fn `UserConstructionScript`)