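; BP_AICharacter is an enemy character that chases the player and can be killed by damage.
; Overlapping Sphere1 with BP_CharacterNEW tells BP_AIController to move to the character while movement is active, and leaving it stops the chase.
; AnyDamage lowers health with debug prints; at zero it deactivates movement, stops the controller and plays a dying sound at world origin.
; ReturnEnemyName just passes through the parent's result.
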(event `self.ReceiveAnyDamage`
  (params (Damage :type "Float (single-precision)") (DamageType :type "DamageType Object Reference") (InstigatedBy :type "Controller Object Reference") (DamageCauser :type "Actor Object Reference"))
  (bind _healspoints (`self.HealsPoints`))
  (if (> _healspoints 0.0)
    (bind _output_get (set `self.HealsPoints` (- _healspoints Damage)))
    (if (> (`self.HealsPoints`) 0.0)
      (`KismetSystemLibrary.PrintString` (`KismetStringLibrary.Concat_StrStr` "HOLLY SHIT I HAVE" (`KismetStringLibrary.Conv_DoubleToString` _output_get) " HP LEFT") true true (struct :`R` 1.0 :`G` 0.652327 :`B` 0.702251 :`A` 1.0) 200.0)
      (else
        (`KismetSystemLibrary.PrintString` "ALWAYS MUST BE KING-CUBE" true true (struct :`R` 0.38947 :`G` 1.0 :`B` 0.357114 :`A` 1.0) 10.0)
        (`ActorComponent.SetActive` (`self.CharacterMovement`) false false)
        (`Controller.StopMovement` (cast `/Game/Бегающий_столб(AI)/BP_AIController` (`self.GetController`) :!pure true))
        (`GameplayStatics.PlaySoundAtLocation` "/Game/Sounds/DyingZombie.DyingZombie" (0.0 0.0 0.0) (struct) 1.0 1.0 0.0 null null null)))))

(event `self.Sphere1.OnComponentBeginOverlap`
  (params (OverlappedComponent :type "PrimitiveComponent Object Reference") (OtherActor :type "Actor Object Reference") (OtherComp :type "PrimitiveComponent Object Reference") (OtherBodyIndex :type Integer) (bFromSweep :type Boolean) (SweepResult :type "HitResult Structure (by ref)"))
  (cast `/Game/Character/BP_CharacterNEW` OtherActor)
  (if (`ActorComponent.IsActive` (`self.CharacterMovement`))
    (`/Game/Бегающий_столб(AI)/BP_AIController.move to the character ` (cast `/Game/Бегающий_столб(AI)/BP_AIController` (`self.GetController`) :!pure true) 5.0)))

(event `self.Sphere1.OnComponentEndOverlap`
  (params (OverlappedComponent :type "PrimitiveComponent Object Reference") (OtherActor :type "Actor Object Reference") (OtherComp :type "PrimitiveComponent Object Reference") (OtherBodyIndex :type Integer))
  (cast `/Game/Character/BP_CharacterNEW` OtherActor)
  (`Controller.StopMovement` (cast `/Game/Бегающий_столб(AI)/BP_AIController` (`self.GetController`) :!pure true)))

(fn `ReturnEnemyName`
  (returns (Name :type Text))
  (bind _name (`parent.ReturnEnemyName`))
  (return _name))

(fn `UserConstructionScript`)