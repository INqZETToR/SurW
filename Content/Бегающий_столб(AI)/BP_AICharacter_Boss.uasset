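; Boss enemy AI character that chases the player character while it is inside a detection sphere.
; Sphere overlap tells BP_AIController to move to the character, provided movement is active, and end overlap stops that movement.
; Health and name getters report HP as a fraction of max and pass the parent's enemy name through, with a leftover NewFunction_0 returning the parent's HP percent.
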(event `self.Sphere123.OnComponentBeginOverlap`
  (params (OverlappedComponent :type "PrimitiveComponent Object Reference") (OtherActor :type "Actor Object Reference") (OtherComp :type "PrimitiveComponent Object Reference") (OtherBodyIndex :type Integer) (bFromSweep :type Boolean) (SweepResult :type "HitResult Structure (by ref)"))
  (cast `/Game/Character/BP_CharacterNEW` OtherActor)
  (if (`ActorComponent.IsActive` (`self.CharacterMovement`))
    (`/Game/Бегающий_столб(AI)/BP_AIController.move to the character ` (cast `/Game/Бегающий_столб(AI)/BP_AIController` (`self.GetController`) :!pure true) 5.0)))

(event `self.Sphere123.OnComponentEndOverlap`
  (params (OverlappedComponent :type "PrimitiveComponent Object Reference") (OtherActor :type "Actor Object Reference") (OtherComp :type "PrimitiveComponent Object Reference") (OtherBodyIndex :type Integer))
  (cast `/Game/Character/BP_CharacterNEW` OtherActor)
  (bind _asbp_aicontroller (cast `/Game/Бегающий_столб(AI)/BP_AIController` (`self.GetController`)))
  (`Controller.StopMovement` _asbp_aicontroller))

(fn `NewFunction_0`
  (returns (Perc :type "Float (double-precision)"))
  (bind _perc (`parent.ReturnHPinPercent`))
  (return _perc))

(fn `ReturnEnemyName`
  (returns (Name :type Text))
  (bind _name (`parent.ReturnEnemyName`))
  (return _name))

(fn `ReturnHPinPercent`
  (returns (Perc :type "Float (double-precision)"))
  (return (/ (`self.HealsPoints`) (`self.MaxHP`))))

(fn `UserConstructionScript`)