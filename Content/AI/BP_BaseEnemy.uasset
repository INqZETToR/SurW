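; BP_BaseEnemy is the base zombie enemy, tracking health and exposing its health fraction and name through getters.
; AnyDamage subtracts health and, on death, stops movement, disables capsule collision, plays death effects and updates the player's kill counter and widget.
; Reaching the player's kill threshold spawns the boss.
; The base casts itself to the boss class to play victory sounds and show the victory widget when the boss dies.
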(event `self.ReceiveBeginPlay`
  (set `self.HealsPoints` (`self.MaxHP`)))

(event `self.ReceiveAnyDamage`
  (params (Damage :type "Float (single-precision)") (DamageType :type "DamageType Object Reference") (InstigatedBy :type "Controller Object Reference") (DamageCauser :type "Actor Object Reference"))
  (bind _healspoints (`self.HealsPoints`))
  (bind _asbp_character_new (cast `/Game/Character/BP_CharacterNEW` (`GameplayStatics.GetPlayerCharacter` 0) :!pure true))
  (bind _countofkills (`/Game/Character/BP_CharacterNEW.CountOfKills` _asbp_character_new))
  (if (> _healspoints 0.0)
    (set `self.HealsPoints` (- _healspoints Damage))
    (if (not (> (`self.HealsPoints`) 0.0))
      (cast `/Game/AI/BP_AICharacter_Boss` self
        (:`then`
          (`GameplayStatics.SpawnSoundAtLocation` "/Game/Sounds/Victory2.Victory2" (0.0 0.0 0.0) (struct) 1.0 1.0 0.0 null null)
          (`KismetSystemLibrary.Delay` 0.5)
          (`GameplayStatics.SpawnSoundAtLocation` "/Game/Sounds/Victory1.Victory1" (0.0 0.0 0.0) (struct) 1.0 1.0 0.0 null null)
          (bind _returnvalue (`|CreateWidget` "/Game/HUD/GameVictoryWidget.GameVictoryWidget_C"))
          (`UserWidget.AddToViewport` _returnvalue 0))
        (:`CastFailed`
          _))
      (set `self.IsDead` true)
      (`ActorComponent.SetActive` (`self.CharacterMovement`) false false)
      (`Controller.StopMovement` (cast `/Game/AI/BP_AIController` (`self.GetController`) :!pure true))
      (`PrimitiveComponent.SetCollisionEnabled` (`self.CapsuleComponent`) "NoCollision")
      (`SkeletalMeshComponent.PlayAnimation` (`self.Mesh`) "/Game/ZombieAssets/zombieAnimations/Zombie_Z_FallingForward.Zombie_Z_FallingForward" false)
      (`GameplayStatics.PlaySoundAtLocation` "/Game/Sounds/DyingZombie.DyingZombie" (0.0 0.0 0.0) (struct) 1.0 1.0 0.0 null null null)
      (`/Engine/EditorBlueprintResources/StandardMacros.IncrementInt` _countofkills
        (:`  `
          (`/Game/HUD/MainWidget.UpdateZombiesKilledCount` (`/Game/Character/BP_CharacterNEW.MWidget` _asbp_character_new))
          (if (== _countofkills (`/Game/Character/BP_CharacterNEW.CountOfZombiesForBossFight` _asbp_character_new))
            (`AIBlueprintHelperLibrary.SpawnAIFromClass` "/Game/AI/BP_AICharacter_Boss.BP_AICharacter_Boss_C" null (0.0 1500.0 0.0) (struct :`Yaw` 270.0))
            (`GameplayStatics.PlaySoundAtLocation` "/Game/Sounds/MainBoss.MainBoss" (0.0 0.0 0.0) (struct) 1.5 1.0 0.0 null null null)))))))

(fn `ReturnEnemyName`
  (returns (Name :type Text))
  (return (`self.Name`)))

(fn `ReturnHPinPercent`
  (returns (Perc :type "Float (double-precision)"))
  (return (/ (`self.HealsPoints`) (`self.MaxHP`))))

(fn `UserConstructionScript`)