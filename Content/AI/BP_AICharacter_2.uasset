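; AI enemy character that chases the player character and can fire a projectile as a ranged attack.
; Sphere1 overlaps with BP_CharacterNEW make its BP_AIController start moving toward the character, if movement is active, or stop when the overlap ends.
; RangeAttack spawns a projectile at ShootPoint and pushes its sphere with a local-space force.
; Helper functions expose health percentage and the parent's enemy name.
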(event `self.Sphere1.OnComponentBeginOverlap`
  (params (OverlappedComponent :type "PrimitiveComponent Object Reference") (OtherActor :type "Actor Object Reference") (OtherComp :type "PrimitiveComponent Object Reference") (OtherBodyIndex :type Integer) (bFromSweep :type Boolean) (SweepResult :type "HitResult Structure (by ref)"))
  (cast `/Game/Character/BP_CharacterNEW` OtherActor)
  (if (`ActorComponent.IsActive` (`self.CharacterMovement`))
    (`/Game/AI/BP_AIController.move to the character ` (cast `/Game/AI/BP_AIController` (`self.GetController`) :!pure true) 500.0)))

(event `self.Sphere1.OnComponentEndOverlap`
  (params (OverlappedComponent :type "PrimitiveComponent Object Reference") (OtherActor :type "Actor Object Reference") (OtherComp :type "PrimitiveComponent Object Reference") (OtherBodyIndex :type Integer))
  (cast `/Game/Character/BP_CharacterNEW` OtherActor)
  (`Controller.StopMovement` (cast `/Game/AI/BP_AIController` (`self.GetController`) :!pure true)))

(event `RangeAttack`
  (bind _returnvalue (`|SpawnActorFromClass` "/Game/AI/ProjectileForRangeAttack.ProjectileForRangeAttack_C" (`SceneComponent.K2_GetComponentToWorld` (`self.ShootPoint`)) "Undefined" "OverrideRootScale" self null))
  (`PrimitiveComponent.AddForceAtLocationLocal` (`/Game/AI/ProjectileForRangeAttack.Sphere` _returnvalue) (0.0 1000.0 0.0) (0.0 0.0 0.0) "None"))

(fn `NewFunction_0`
  (returns (Perc :type "Float (double-precision)"))
  (bind _perc (`parent.ReturnHPinPercent`))
  (return _perc))

(fn `ReturnEnemyName`
  (returns (Name :type Text))
  (bind _name (`parent.ReturnEnemyName`))
  (return _name))

(fn `ReturnHPinPercent`
  (returns (Perc :type "Float (double-precision)"))
  (return (/ (`self.HealsPoints`) (`self.MaxHP`))))

(fn `UserConstructionScript`)