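; BP_AICharacter is an AI-controlled enemy that chases the player character while it is within a detection sphere.
; Sphere1 begin overlap with BP_CharacterNEW tells BP_AIController to move to the character, provided CharacterMovement is active.
; End overlap tells the controller to stop movement.
; The ReturnEnemyName override simply returns the parent's result.
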(event `self.Sphere1.OnComponentBeginOverlap`
  (params (OverlappedComponent :type "PrimitiveComponent Object Reference") (OtherActor :type "Actor Object Reference") (OtherComp :type "PrimitiveComponent Object Reference") (OtherBodyIndex :type Integer) (bFromSweep :type Boolean) (SweepResult :type "HitResult Structure (by ref)"))
  (cast `/Game/Character/BP_CharacterNEW` OtherActor)
  (if (`ActorComponent.IsActive` (`self.CharacterMovement`))
    (`/Game/AI/BP_AIController.move to the character ` (cast `/Game/AI/BP_AIController` (`self.GetController`) :!pure true) 5.0)))

(event `self.Sphere1.OnComponentEndOverlap`
  (params (OverlappedComponent :type "PrimitiveComponent Object Reference") (OtherActor :type "Actor Object Reference") (OtherComp :type "PrimitiveComponent Object Reference") (OtherBodyIndex :type Integer))
  (cast `/Game/Character/BP_CharacterNEW` OtherActor)
  (`Controller.StopMovement` (cast `/Game/AI/BP_AIController` (`self.GetController`) :!pure true)))

(fn `ReturnEnemyName`
  (returns (Name :type Text))
  (bind _name (`parent.ReturnEnemyName`))
  (return _name))

(fn `UserConstructionScript`)