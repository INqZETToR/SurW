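; Base melee weapon that damages enemies caught in a fan-shaped sweep in front of its DamagePoint.
; Attack yaws DamagePoint across the rotation range in small steps, firing three pitch-offset Visibility line traces at each step with persistent debug drawing.
; Hit actors are cast to BP_BaseEnemy and gathered uniquely, then the point's rotation resets and an event applies Damage to each gathered entry.
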(event `deal damage to attacked enemies`
  (params (enemies :type "Array of /Game/Бегающий_столб(AI)/BP_BaseEnemy Object Reference"))
  (for _array_element enemies
    (`GameplayStatics.ApplyDamage` _array_element (`self.Damage`))))

(fn `Attack`
  (locals (L_rotation :type "Float (double-precision)") (damagedEnemies :type "Array of /Game/Бегающий_столб(AI)/BP_BaseEnemy Object Reference"))
  (bind _damagepoint (`self.damagePoint`))
  (bind _returnvalue (`SceneComponent.K2_GetComponentLocation` _damagepoint))
  (bind _returnvalue_2 (- 0.0 (`self.MaxRotateRange`)))
  (bind _returnvalue_3 (+ _returnvalue (* (`SceneComponent.GetForwardVector` _damagepoint) (`self.MaxAttackRange`))))
  ;[1 1 1] под углом изза поворота ножа
  (set `local.L_rotation` _returnvalue_2)
  (`SceneComponent.K2_AddLocalRotation` (`self.damagePoint`) (`KismetMathLibrary.MakeRotator` 0.0 0.0 _returnvalue_2) false false)
  (while (>= (`self.MaxRotateRange`) (`local.L_rotation`))
    (`|ExecutionSequence`
      (:`then_0`
        (bind (_outhit _returnvalue_4) (`KismetSystemLibrary.LineTraceSingle` :`Start` _returnvalue :`End` _returnvalue_3 :`TraceChannel` "TraceTypeQuery1" :`bTraceComplex` true :`DrawDebugType` "Persistent"))
        (`SceneComponent.K2_AddLocalRotation` (`self.damagePoint`) (`KismetMathLibrary.MakeRotator` 0.0 5.0 0.0) false false))
      (:`then_1`
        (bind (_outhit_2 _returnvalue_5) (`KismetSystemLibrary.LineTraceSingle` :`Start` _returnvalue :`End` _returnvalue_3 :`TraceChannel` "TraceTypeQuery1" :`bTraceComplex` true :`DrawDebugType` "Persistent"))
        (`SceneComponent.K2_AddLocalRotation` (`self.damagePoint`) (`KismetMathLibrary.MakeRotator` 0.0 -10.0) false false))
      (:`then_2`
        (bind (_outhit_3 _returnvalue_6) (`KismetSystemLibrary.LineTraceSingle` :`Start` _returnvalue :`End` _returnvalue_3 :`TraceChannel` "TraceTypeQuery1" :`bTraceComplex` true :`DrawDebugType` "Persistent"))
        (set `local.L_rotation` (+ (`local.L_rotation`) 5.0))
        (`SceneComponent.K2_AddLocalRotation` (`self.damagePoint`) (`KismetMathLibrary.MakeRotator` 0.0 5.0 5.0) false false))
      (:`then_3`
        (`|ExecutionSequence`
          (:`then_0`
            (if _returnvalue_4
              (`KismetArrayLibrary.Array_AddUnique` (`local.damagedEnemies`) (cast `/Game/Бегающий_столб(AI)/BP_BaseEnemy` (`.HitActor` (`GameplayStatics.BreakHitResult` _outhit)) :!pure true))))
          (:`then_1`
            (if _returnvalue_5
              (`KismetArrayLibrary.Array_AddUnique` (`local.damagedEnemies`) (cast `/Game/Бегающий_столб(AI)/BP_BaseEnemy` (`.HitActor` (`GameplayStatics.BreakHitResult` _outhit_2)) :!pure true))))
          (:`then_2`
            (if _returnvalue_6
              (`KismetArrayLibrary.Array_AddUnique` (`local.damagedEnemies`) (cast `/Game/Бегающий_столб(AI)/BP_BaseEnemy` (`.HitActor` (`GameplayStatics.BreakHitResult` _outhit_3)) :!pure true))))))))
  ;;[1 1 1] как это работаит?
  (`SceneComponent.K2_SetRelativeRotation` :`self` (`self.damagePoint`))
  (`self.deal damage to attacked enemies` (`local.damagedEnemies`)))

(fn `UserConstructionScript`)