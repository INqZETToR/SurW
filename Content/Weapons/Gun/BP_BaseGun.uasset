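; BP_BaseGun is a gun Blueprint that handles firing and reloading for the player's BP_CharacterNEW.
; Shoot decrements the equipped gun's ammo, spawns a physics-propelled bullet at ShootPoint and adds recoil through random yaw and fixed pitch controller input.
; The auto-reload event waits ReloadTime, refills the magazine from the character's TotalAmmo or flags NoAmmo, and updates the ammo widget.
; Both sounds play at world origin.
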(event `auto-reload`
  (bind _asbp_character_new (cast `/Game/Character/BP_CharacterNEW` (`GameplayStatics.GetPlayerCharacter` 0) :!pure true))
  (bind _asbp_character_new_2 (cast `/Game/Character/BP_CharacterNEW` (`GameplayStatics.GetPlayerCharacter` 0) :!pure true))
  (bind _asbp_character_new_3 (cast `/Game/Character/BP_CharacterNEW` (`GameplayStatics.GetPlayerCharacter` 0) :!pure true))
  (bind _totalammo (`/Game/Character/BP_CharacterNEW.TotalAmmo` _asbp_character_new))
  (bind _mwidget (`/Game/Character/BP_CharacterNEW.MWidget` _asbp_character_new_2))
  (`/Game/HUD/MainWidget.DoAmmoTextReloading` (`/Game/Character/BP_CharacterNEW.MWidget` _asbp_character_new_3))
  (if (!= (`/Game/Character/BP_CharacterNEW.TotalAmmo` _asbp_character_new) 0)
    (`KismetSystemLibrary.Delay` (`self.ReloadTime`))
    (if (> (`/Game/Character/BP_CharacterNEW.TotalAmmo` _asbp_character_new) (`self.AmmoInWeapon`))
      (set `self.CurrentAmmoInWeapon` (`self.AmmoInWeapon`))
      (set `/Game/Character/BP_CharacterNEW.TotalAmmo` (- _totalammo (`self.AmmoInWeapon`)) _asbp_character_new)
      (set `/Game/Character/BP_CharacterNEW.CanShoot` true _asbp_character_new)
      (else
        (set `self.CurrentAmmoInWeapon` _totalammo)
        (set `/Game/Character/BP_CharacterNEW.TotalAmmo` 0 _asbp_character_new)
        (set `/Game/Character/BP_CharacterNEW.CanShoot` true _asbp_character_new)))
    (`GameplayStatics.PlaySoundAtLocation` "/Game/Sounds/reload.reload" (0.0 0.0 0.0) (struct) 1.0 1.0 0.0 null null null)
    (else
      (set `/Game/Character/BP_CharacterNEW.NoAmmo?` true _asbp_character_new_3)))
  (`/Game/HUD/MainWidget.UndoAmmoTextReloading` _mwidget)
  (`/Game/HUD/MainWidget.UpdateAmmoCount` _mwidget (`/Game/Weapons/Gun/BP_BaseGun.CurrentAmmoInWeapon` (`/Game/Character/BP_CharacterNEW.EqGun` _asbp_character_new_2)) (`/Game/Character/BP_CharacterNEW.TotalAmmo` _asbp_character_new_2)))

(fn `Shoot`
  (bind _asbp_character_new (cast `/Game/Character/BP_CharacterNEW` (`GameplayStatics.GetPlayerCharacter` 0) :!pure true))
  (`/Engine/EditorBlueprintResources/StandardMacros.DecrementInt` (`/Game/Weapons/Gun/BP_BaseGun.CurrentAmmoInWeapon` (`/Game/Character/BP_CharacterNEW.EqGun` (cast `/Game/Character/BP_CharacterNEW` (`GameplayStatics.GetPlayerCharacter` 0) :!pure true)))
    (:`  `
      (`GameplayStatics.PlaySoundAtLocation` "/Game/Sounds/shot.shot" (0.0 0.0 0.0) (struct) 1.0 1.0 0.0 null null null)
      (bind _returnvalue (`|SpawnActorFromClass` "/Game/Weapons/Bullet.Bullet_C" (`SceneComponent.K2_GetComponentToWorld` (`self.ShootPoint`)) "Undefined" "OverrideRootScale" null null))
      (`PrimitiveComponent.AddForceAtLocationLocal` (`/Game/Weapons/Bullet.Capsule` _returnvalue) (0.0 0.0 -4000.0) (0.0 0.0 0.0) "None")
      ;[1 1 1] spreading while shoot
      (`Pawn.AddControllerYawInput` _asbp_character_new (`KismetMathLibrary.RandomFloatInRange` -0.5 0.5))
      (`Pawn.AddControllerPitchInput` _asbp_character_new (* (`self.SpreadingVal`) -1.0)))))

(fn `UserConstructionScript`)