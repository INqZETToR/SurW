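; BP_A47K is a gun Blueprint that shows its ammo on text render components.
; On BeginPlay it calls the parent logic, sets its own reload time and magazine size, starts fully loaded, and makes both ammo displays visible.
; Its RefreshTextRenders event writes the current magazine count and the total ammo, read by casting player zero's character to BP_CharacterNEW.
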(event `refresh text renders`
  (`TextRenderComponent.K2_SetText` (`self.AmmoInWeapon_TextRender`) (`KismetTextLibrary.Conv_IntToText` (`self.CurrentAmmoInWeapon`)))
  (`TextRenderComponent.K2_SetText` (`self.TotalAmmo_TextRender`) (`KismetTextLibrary.Conv_IntToText` (`/Game/Character/BP_CharacterNEW.TotalAmmo` (cast `/Game/Character/BP_CharacterNEW` (`GameplayStatics.GetPlayerCharacter` 0) :!pure true)))))

(event `self.ReceiveBeginPlay`
  (`parent.ReceiveBeginPlay`)
  (set `self.ReloadTime` 3.0)
  (set `self.AmmoInWeapon` 30)
  (set `self.CurrentAmmoInWeapon` 30)
  (`self.refresh text renders`)
  (`SceneComponent.SetVisibility` (`self.AmmoInWeapon_TextRender`) true false)
  (`SceneComponent.SetVisibility` (`self.TotalAmmo_TextRender`) true false))

(fn `UserConstructionScript`
  (`parent.UserConstructionScript`))