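; BP_PickUpActor is a world pickup that adds an item to the inventory of an overlapping BP_CharacterNEW.
; On BeginPlay it applies its configured mesh and material to Sphere2 once, guarded by a flag.
; Sphere overlap passes ItemClass and Amount to the character's InventoryRef.
; The actor destroys itself on success or when a failed add leaves no remainder, otherwise it keeps the leftover as its new Amount.
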(event `self.ReceiveBeginPlay`
  (if (not (`self.SettedYet?`))
    (`StaticMeshComponent.SetStaticMesh` (`self.Sphere2`) (`self.StatMesh`))
    (`PrimitiveComponent.SetMaterial` (`self.Sphere2`) 0 (`self.Mater`))
    (set `self.SettedYet?` true)))

(event `self.Sphere.OnComponentBeginOverlap`
  (params (OverlappedComponent :type "PrimitiveComponent Object Reference") (OtherActor :type "Actor Object Reference") (OtherComp :type "PrimitiveComponent Object Reference") (OtherBodyIndex :type Integer) (bFromSweep :type Boolean) (SweepResult :type "HitResult Structure (by ref)"))
  ;[1 1 1] Overlaping
  (bind _asbp_character_new (cast `/Game/Character/BP_CharacterNEW` OtherActor))
  (bind _inventoryref (`/Game/Character/BP_CharacterNEW.InventoryRef` _asbp_character_new))
  (`/Engine/EditorBlueprintResources/StandardMacros.IsValid` _inventoryref
    (:`Is Valid`
      (bind (_success_ _rest) (`/Game/InventorySystem/Blueprints/BP_Inventory.AddItem` _inventoryref (`self.Amount`) (`self.ItemClass`)))
      (if _success_
        (`self.K2_DestroyActor` :!label _label)
        (elif (> _rest 0)
          (set `self.Amount` _rest)
          (else
            (goto _label)))))))

(fn `UserConstructionScript`)