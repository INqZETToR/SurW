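; ItemHealPotion is an inventory item Blueprint for a healing potion.
; Its Use event calls Heal on the given player with the HealCount amount, then prints the player's HP to screen.
; BeginPlay, overlap and Tick are left as disabled default nodes, and the construction script only calls its parent.
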(event `self.Use`
  (params (Player :type "/Game/Character/BP_CharacterNEW Object Reference"))
  (`/Game/Character/BP_CharacterNEW.Heal` Player (`self.HealCount`))
  (`KismetSystemLibrary.PrintString` (`KismetStringLibrary.Conv_DoubleToString` (`/Game/Character/BP_CharacterNEW.HP` Player))))

(fn `UserConstructionScript`
  (`parent.UserConstructionScript`))