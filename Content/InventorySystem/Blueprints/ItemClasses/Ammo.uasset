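; Ammo item Blueprint for the inventory system that tops up the player's ammunition when used.
; Its Use event adds the item's AmmoCount to the player's TotalAmmo, then calls RefreshTextRend on the player to refresh the display.
; All other graph logic is just disabled default events and a construction script that calls its parent.
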(event `self.Use`
  (params (Player :type "/Game/Character/BP_CharacterNEW Object Reference"))
  (set `/Game/Character/BP_CharacterNEW.TotalAmmo` (+ (`self.AmmoCount`) (`/Game/Character/BP_CharacterNEW.TotalAmmo` Player)) Player)
  (`/Game/Character/BP_CharacterNEW.RefreshTextRend` Player))

(fn `UserConstructionScript`
  (`parent.UserConstructionScript`))