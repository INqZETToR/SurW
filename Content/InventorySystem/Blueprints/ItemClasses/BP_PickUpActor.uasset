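; BP_PickUpActor is a world pickup that adds an item to the player's inventory when BP_CharacterNEW overlaps its sphere.
; On overlap it calls AddItem on the character's InventoryRef with its ItemClass and Amount.
; It destroys itself when the add succeeds or nothing remains, and otherwise keeps the leftover count as its new Amount for a later pickup.
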(event `self.Sphere.OnComponentBeginOverlap`
  (params (OverlappedComponent :type "PrimitiveComponent Object Reference") (OtherActor :type "Actor Object Reference") (OtherComp :type "PrimitiveComponent Object Reference") (OtherBodyIndex :type Integer) (bFromSweep :type Boolean) (SweepResult :type "HitResult Structure (by ref)"))
  (bind _asbp_character_new (cast `/Game/Character/BP_CharacterNEW` OtherActor))
  (bind _inventoryref (`/Game/Character/BP_CharacterNEW.InventoryRef` _asbp_character_new))
  (`/Engine/EditorBlueprintResources/StandardMacros.IsValid` _inventoryref
    (:`Is Valid`
      (bind (_success_ _rest) (`/Game/InventorySystem/Blueprints/BP_Inventory.AddItem` _inventoryref (`self.Amount`) (`self.ItemClass`)))
      (if _success_
        (`self.K2_DestroyActor` :!label _label)
        (elif (> _rest 0)
          (set `self.Amount` _rest)
          (else
            (goto _label)))))))

(fn `UserConstructionScript`)